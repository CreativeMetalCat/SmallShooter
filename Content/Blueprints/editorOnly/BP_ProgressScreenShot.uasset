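; Editor-only progress screenshot tool that, when TakePictures is on, photographs the level from a list of cameras at BeginPlay.
; It has the player controller possess it, then loops through Cameras with a view-target blend and delays around each high-res 1080p screenshot.
; Images save to an OldTown_Progress folder under the project user directory, organised by level name and version and named per camera.
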(event EventBeginPlay
  (bind _returnvalue (Game|GetPlayerController 0))
  (bind _cameras (Variables|Default|GetCameras))
  (bind _currentcameraid (Variables|Default|GetCurrentCameraId))
  (bind _output (Utilities|Array|Get(acopy) _cameras _currentcameraid))
  (if (Variables|Default|GetTakePictures)
    (Pawn|Possess _returnvalue self)
    (bind _returnvalue_2 (Game|GetCurrentLevelName true))
    (bind _output_get (Variables|Default|SetLevelName _returnvalue_2))
    (if (Utilities|Array|IsValidIndex _cameras _currentcameraid) :!label _label
      (Game|Player|SetViewTargetwithBlend _returnvalue 0 0.5 "VTBlend_Linear" 0.0 false)
      (Utilities|FlowControl|Delay 0.5)
      (Class|AutomationBlueprintFunctionLibrary|TakeHighResScreenshot 1920 1080 (Utilities|String|Append (Class|BlueprintPathsLibrary|ProjectUserDir) "/OldTown_Progress/" (Utilities|String|Append _output_get (Utilities|String|ToString(Integer) (Variables|Default|Getversion)) "/" _output_get "_" (Utilities|GetDisplayName _output))) _output false false "Low" "" 0.0)
      (Utilities|FlowControl|Delay 0.2)
      (Development|PrintString "PictureTaken")
      (Math|Integer|IncrementInt (Variables|Default|GetCurrentCameraId)
        (:%20%20
          (goto _label))))))

(fn ConstructionScript)