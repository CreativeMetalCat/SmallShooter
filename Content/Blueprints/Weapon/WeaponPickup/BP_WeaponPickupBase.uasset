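; Base weapon pickup actor that shows a weapon in the world and hands it to actors that walk into it.
; On BeginPlay it looks up its weapon row in a data table and shows either a static or skeletal mesh based on that data.
; On capsule overlap it passes the weapon data through BPI_Interaction and destroys itself if the pickup is accepted.
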(event OnComponentBeginOverlap(Capsule)
  (params (OverlappedComponent :type Primitive%20Component%20Object%20Reference) (OtherActor :type Actor%20Object%20Reference) (OtherComp :type Primitive%20Component%20Object%20Reference) (OtherBodyIndex :type Integer) (bFromSweep :type Boolean) (SweepResult :type Hit%20Result%20Structure%20%28by%20ref%29))
  (if (Utilities|DoesObjectImplementInterface OtherActor "/Game/Blueprints/BPI_Interaction.BPI_Interaction_C")
    (bind _pickedup (Class|BPIInteraction|PickUpWeapon(Message) OtherActor (Variables|SPAWN_ONLY|GetWeaponData)))
    (if _pickedup
      (Actor|DestroyActor))))

(event EventBeginPlay
  (bind _weapon (Variables|Default|GetWeapon))
  (bind _weaponmesh_skeletal (Variables|Default|GetWeaponMesh_Skeletal))
  (bind _weaponmesh_static (Variables|Default|GetWeaponMesh_Static))
  (bind (_datatable _rowname) (Utilities|Struct|BreakDataTableRowHandle _weapon))
  (bind _returnvalue (Utilities|GetDataTableRow _datatable _rowname)
    (:then
      (bind _output_get (Variables|SPAWN_ONLY|SetWeaponData _returnvalue))
      (if (.UsesStaticMesh (Utilities|Struct|BreakS_Weapon _output_get))
        (Components|StaticMesh|SetStaticMesh _weaponmesh_static (.StaticMesh (Utilities|Struct|BreakS_Weapon _output_get)))
        (Rendering|SetVisibility _weaponmesh_static true false)
        (Rendering|SetVisibility (Variables|Default|GetWeaponMesh_Skeletal) false false)
        (else
          (Class|SkinnedMeshComponent|SetSkeletalMesh _weaponmesh_skeletal (.Mesh (Utilities|Struct|BreakS_Weapon _output_get)) true)
          (Rendering|SetVisibility _weaponmesh_skeletal true false)
          (Rendering|SetVisibility (Variables|Default|GetWeaponMesh_Static) false false))))))

(event Collision|EventActorBeginOverlap
  (params (OtherActor :type Actor%20Object%20Reference)))

(event EventTick
  (params (DeltaSeconds :type Float%20%28single-precision%29)))

(fn ConstructionScript)