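; Shotgun fire component for weapons that spawns a spread of bullet actors per shot.
; Fire loops over Amount, aiming each bullet along a random direction in a Spread-wide cone around the supplied rotation, reseeding WeaponRandomStream each time.
; Each bullet receives Damage and the component's owner, which its collision ignores while moving.
; The BulletClass input is unused, as the spawn class is fixed to BP_Bullet.
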(event EventBeginPlay
  (|CallParentFunction) ; This node is disabled and will not be called.\nDrag off pins to build functionality.
)

(event EventTick
  (params (DeltaSeconds :type Float%20%28single-precision%29))
  (|CallParentFunction DeltaSeconds) ; This node is disabled and will not be called.\nDrag off pins to build functionality.
)

(fn Fire
  (params (Location :type Vector :default "0, 0, 0") (Rotation :type Rotator :default "0, 0, 0") (BulletClass :type BP%20Bullet%20Class%20Reference) (Damage :type Float%20%28single-precision%29))
  (bind _returnvalue (Components|GetOwner))
  (bind _weaponrandomstream (Variables|Default|GetWeaponRandomStream))
  (for _index (range 0 (Variables|Default|GetAmount))
    (Math|Random|SetRandomStreamSeed _weaponrandomstream (Math|Random|RandomInteger 32767))
    (bind _returnvalue_2 (Game|SpawnActorfromClass "/Game/Blueprints/Projectile/BP_Bullet.BP_Bullet_C" (Math|Transform|MakeTransform Location (Math|Rotator|FindLookatRotation Location (+ (* (Class|KismetMathLibrary|RandomUnitVectorinConeinRadiansfromStream (Math|Rotator|GetRotationXVector Rotation) (Math|Trig|DegreesToRadians (* (Variables|Default|GetSpread) 0.5)) _weaponrandomstream) 1e+02) Location)) "1.000000,1,1") "AlwaysSpawn" _returnvalue Damage 0))
    (Utilities|IsValid _returnvalue_2
      (:Is%20Valid
        (Collision|IgnoreActorwhenMoving (Variables|/Game/Blueprints/Projectile/BP_Bullet.BP_Bullet_C|GetCollisionComponent _returnvalue_2) _returnvalue true)))))