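; BP_Button is an interactable puzzle button that notifies listeners when used and can be limited to a single use.
; Interact waits a configurable delay, then, if not already used, fires the OnInteracted dispatcher with itself and the interactor and plays its sound.
; When OneUse is set, that press latches HasBeenUsed to block later ones.
; The physics-material and pickup functions are empty stubs returning defaults.
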(event EventBeginPlay)

(event Collision|EventActorBeginOverlap
  (params (OtherActor :type Actor%20Object%20Reference)))

(event EventTick
  (params (DeltaSeconds :type Float%20%28single-precision%29)))

(event EventInteract
  (params (Interactor :type Actor%20Object%20Reference) (InteractedComponent :type Scene%20Component%20Object%20Reference))
  (Utilities|FlowControl|Delay (Variables|Default|GetDelay))
  (if (not (Variables|Default|GetHasBeenUsed))
    (Default|CallOnInteracted self Interactor)
    (Audio|Components|Audio|Play (Variables|Default|GetButtonUseSound) 0.0)
    (if (Variables|Default|GetOneUse?)
      (Variables|Default|SetHasBeenUsed true))))

(fn ConstructionScript)

(fn GetPhysicsEffectMaterial
  (return 0))

(fn PickUpAmmo
  (params (Type :type E_AmmoType%20Enum :default "NewEnumerator0") (Amount :type Integer))
  (return false))

(fn PickUpHealth
  (params (Health :type Float%20%28single-precision%29))
  (return false))

(fn PickUpHealthItem
  (params (Size :type Integer))
  (return false))

(fn PickUpWeapon
  (params (Weapon :type S%20Weapon%20Structure))
  (return false))