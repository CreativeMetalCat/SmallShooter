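; Health pickup actor in three sizes, either handed over as an item or applied directly as health.
; The construction script picks the static mesh from Size.
; On box overlap with a BPI_Interaction implementer, the Item flag chooses between sending Size as an item and sending a health amount scaled by Size.
; The pickup destroys itself only when the overlapping actor's interface call returns true.
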(event OnComponentBeginOverlap(Box)
  (params (OverlappedComponent :type Primitive%20Component%20Object%20Reference) (OtherActor :type Actor%20Object%20Reference) (OtherComp :type Primitive%20Component%20Object%20Reference) (OtherBodyIndex :type Integer) (bFromSweep :type Boolean) (SweepResult :type Hit%20Result%20Structure%20%28by%20ref%29))
  (bind _size (Variables|Default|GetSize))
  (if (Utilities|DoesObjectImplementInterface OtherActor "/Game/Blueprints/BPI_Interaction.BPI_Interaction_C")
    (if (Variables|Type|GetItem?)
      (bind _success (Class|BPIInteraction|PickUpHealthItem(Message) OtherActor _size))
      (if _success
        (Actor|DestroyActor))
      (else
        (bind _success_2 (Class|BPIInteraction|PickUpHealth(Message) OtherActor (* (+ _size 1) 15.0)))
        (if _success_2
          (Actor|DestroyActor))))))

(event EventBeginPlay)

(event Collision|EventActorBeginOverlap
  (params (OtherActor :type Actor%20Object%20Reference)))

(event EventTick
  (params (DeltaSeconds :type Float%20%28single-precision%29)))

(fn ConstructionScript
  (Components|StaticMesh|SetStaticMesh (Variables|Default|GetStaticMesh) (Utilities|Select :Index (Variables|Default|GetSize) :Option%200 "/Game/Health_Packs/Meshes/Small_HP.Small_HP" :Option%201 "/Game/Health_Packs/Meshes/Medium_HP_Mk2.Medium_HP_Mk2" :Option%202 "/Game/Health_Packs/Meshes/Large_HP.Large_HP")))