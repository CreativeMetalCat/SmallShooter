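; AI controller for zombies that runs the BT_Zombie behavior tree and picks its target through AI Perception.
; Perception updates write sighted actors with an enemy tag to the Blackboard target and set focus, clearing both when sight is lost.
; An existing target is replaced only when it is nearer than the new actor, despite comments intending the opposite.
; The controller destroys itself without a valid pawn; random-wander logic is left disconnected.
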(event OnTargetPerceptionUpdated(AIPerception)
  (params (Actor :type Actor%20Object%20Reference) (Stimulus :type AI%20Stimulus%20Structure))
  (Utilities|IsValid (Pawn|GetControlledPawn)
    (:Is%20Valid
      (CallFunction|UpdatePerception Actor Stimulus))
    (:Is%20Not%20Valid
      (Actor|DestroyActor))))

(event EventBeginPlay
  (bind _returnvalue (AI|RunBehaviorTree "/Game/Blueprints/AI/ZombieAI/BT_Zombie.BT_Zombie"))
  (if _returnvalue
    _))

(event EventTick
  (params (DeltaSeconds :type Float%20%28single-precision%29)))

(fn ConstructionScript)

(fn UpdatePerception
  (params (Actor :type Actor%20Object%20Reference) (Stimulus :type AI%20Stimulus%20Structure))
  (bind _blackboard_targetname (Variables|BlackboardKeys|GetBlackboard_TargetName))
  (bind _blackboard (Variables|Default|GetBlackboard))
  (bind _returnvalue (AI|Components|Blackboard|GetValueasObject _blackboard _blackboard_targetname))
  ;[1 1 1] check if event was caused by lossing sight of target
  (if (== Actor _returnvalue)
    (if (not (Utilities|Array|ContainsItem (Class|AIPerceptionComponent|GetPerceivedActors (Variables|Default|GetAIPerception) "/Script/AIModule.AISense_Sight") (.AsActor (Utilities|Casting|CastToActor _returnvalue))))
      (AI|Components|Blackboard|ClearValue (Variables|Default|GetBlackboard) (Variables|BlackboardKeys|GetBlackboard_TargetName))
      (AI|SetFocus))
    (else
      ;[1 1 1] Check if the actor is an enemy
      (bind _array_element (Utilities|Array|ForEachLoopwithBreak (Variables|Enemy|Tags|GetEnemyTags) :!label _label)
        (:LoopBody
          (if (Utilities|Array|ContainsItem (Variables|/Script/Engine.Actor|GetTags Actor) _array_element)
            (LocalVariables|SetisEnemy true)
            (goto _label Break)))
        (:Completed
          ;[1 1 1] Make sure we still can see the actor
          (if (LocalVariables|GetisEnemy)
            (if (Utilities|Array|ContainsItem (Class|AIPerceptionComponent|GetPerceivedActors (Variables|Default|GetAIPerception) "/Script/AIModule.AISense_Sight") Actor)
              ;[1 1 1] do we have any target right now?
              (Utilities|IsValid (AI|Components|Blackboard|GetValueasObject (Variables|Default|GetBlackboard) (Variables|BlackboardKeys|GetBlackboard_TargetName))
                (:Is%20Valid
                  ;[1 1 1] Set new target
                  (if (< (Class|KismetMathLibrary|VectorDistanceSquared (Transformation|GetActorLocation (.AsActor (Utilities|Casting|CastToActor (AI|Components|Blackboard|GetValueasObject (Variables|Default|GetBlackboard) (Variables|BlackboardKeys|GetBlackboard_TargetName))))) (Transformation|GetActorLocation (Pawn|GetControlledPawn))) (Class|KismetMathLibrary|VectorDistanceSquared (Transformation|GetActorLocation Actor) (Transformation|GetActorLocation (Pawn|GetControlledPawn))))
                    (AI|Components|Blackboard|SetValueasObject (Variables|Default|GetBlackboard) (Variables|BlackboardKeys|GetBlackboard_TargetName) Actor :!label _label_2)
                    (AI|SetFocus Actor)))
                (:Is%20Not%20Valid
                  (goto _label_2))))))))))