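; Zombie enemy character with melee attacks, limb dismemberment and a crawling state.
; Point damage finds the bone nearest the hit, scales damage and tracks per-limb health, hiding destroyed limbs and switching to crawling when one needed for standing is lost.
; Attack montages damage actors overlapping the attack collision on a notify.
; Death enables ragdoll physics, unpossesses the controller, plays a voice sound and adds a delayed impulse for bullet hits.
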(event EventBeginPlay
  (bind _mesh (Variables|Character|GetMesh))
  (if (Variables|Movement|Crawling|GetCrawling)
    (Components|SkinnedMesh|HideBonebyName _mesh "thigh_r" "PBO_Term")
    (Components|SkinnedMesh|HideBonebyName _mesh "thigh_l" "PBO_Term")
    (Movement|Crawling|StartCrawling)))

(event Game|Damage|EventPointDamage
  (params (Damage :type Float%20%28single-precision%29) (DamageType :type Damage%20Type%20Object%20Reference) (HitLocation :type Vector :default "0, 0, 0") (HitNormal :type Vector :default "0, 0, 0") (HitComponent :type Primitive%20Component%20Object%20Reference) (BoneName :type Name :default "None") (ShotFromDirection :type Vector :default "0, 0, 0") (InstigatedBy :type Controller%20Object%20Reference) (DamageCauser :type Actor%20Object%20Reference) (HitInfo :type Hit%20Result%20Structure%20%28by%20ref%29))
  (bind _resultdamage (Damage|CalculateDamage HitLocation Damage))
  (bind _output_get (Variables|Health|SetHealth (- (Variables|Health|GetHealth) _resultdamage)))
  (Animation|Montage|PlayMontage (Variables|Character|GetMesh) "/Game/Polygonmaker/Animations/Undead/Anim_Zombie_hit1_Montage.Anim_Zombie_hit1_Montage"
    (:then
      (if (<= _output_get 0.0)
        (Death|Die)
        (Utilities|Casting|CastToBP_BulletDamage DamageType)
        (Utilities|AddImpluseatLocationwithDelay (* (Transformation|GetVelocity DamageCauser) 2.0) HitLocation 0.01)))))

(event EventAttack
  (Variables|Attack|SetShouldBeAttacking true)
  (if (not (Variables|Attack|GetAttacking))
    (bind _notifyname (Animation|Montage|PlayMontage (Variables|Character|GetMesh) (select (Variables|Movement|Crawling|GetCrawling) "/Game/Polygonmaker/Animations/Undead/Anim_Zombie_ground-attack_Montage.Anim_Zombie_ground-attack_Montage" "/Game/Polygonmaker/Animations/Undead/Anim_Zombie_attack3_Montage.Anim_Zombie_attack3_Montage"))
      (:then
        (Variables|Attack|SetAttacking true))
      (:OnCompleted
        (Variables|Attack|SetAttacking false))
      (:OnNotifyBegin
        (if (Utilities|Name|Equal(Name) _notifyname "Damage")
          (for _array_element (Collision|GetOverlappingActors (Variables|Default|GetAttackCollision) 0 :!class /Script/Engine.PrimitiveComponent)
            (Game|Damage|ApplyDamage _array_element 2e+01 (Pawn|GetController) self)))))))

(fn ConstructionScript)

(fn Die
  (bind _mesh (Variables|Character|GetMesh))
  (if (not (Variables|Health|GetDead))
    (Variables|Health|SetDead true)
    (Collision|SetCollisionEnabled _mesh "PhysicsOnly")
    (Physics|SetSimulatePhysics _mesh true)
    (Collision|SetCollisionEnabled (Variables|Collision|GetCapsuleComponent) "NoCollision")
    (Pawn|UnPossess (Pawn|GetController))
    (CallFunction|PlayVoiceSound (Variables|Sounds|Death|GetDeathSound))))

(fn GetCurrentSpeedRate
  (return (/ (Math|Vector|VectorLength (Transformation|GetVelocity)) (Math|Float|SelectFloat (Variables|Movement|Crawling|GetDefaultCrawlingSpeed) (Variables|Movement|GetDefaultMovementSpeed) (Variables|Movement|Crawling|GetCrawling)))))

(fn CalculateDamage
  (params (HitLocation :type Vector) (Damage :type Float%20%28single-precision%29))
  (bind _mesh (Variables|Character|GetMesh))
  (bind _limbdata (Variables|LimbData|GetLimbData))
  (bind (_bonelocation _returnvalue) (Class|SkinnedMeshComponent|FindClosestBoneK2 _mesh HitLocation 0.0 true))
  (bind _returnvalue_2 (Math|Vector|Distance(Vector) HitLocation _bonelocation))
  (bind _returnvalue_3 (Utilities|String|ToString(Name) _returnvalue))
  (bind (_value _returnvalue_4) (Utilities|Map|Find _limbdata _returnvalue_3))
  (Development|PrintString (Utilities|String|Append (Utilities|String|ToString(Float) _returnvalue_2) " : " (Utilities|String|ToString(Name) _returnvalue)))
  (if (and _returnvalue_4 (<= _returnvalue_2 (Math|Float|SelectFloat 6e+01 34.0 (Variables|Movement|Crawling|GetCrawling))))
    (Damage|CalculateDamage|ApplyLimbDamage Damage _returnvalue_3)
    (return (* Damage (Utilities|Struct|BreakS_LimbData _value)))
    (else
      (return Damage))))

(fn ApplyLimbDamage
  (params (Damage :type Float%20%28single-precision%29) (LimbName :type String))
  (bind _limbhealth (Variables|LimbData|GetLimbHealth))
  (bind _limbdata (Variables|LimbData|GetLimbData))
  (bind (_value _returnvalue) (Utilities|Map|Find _limbhealth LimbName))
  (bind _value_2 (Utilities|Map|Find _limbdata LimbName))
  (bind _limbhealth_2 (Utilities|Struct|BreakS_LimbData _value_2))
  (bind _returnvalue_2 (- _limbhealth_2 Damage))
  (if _returnvalue
    (if (>= Damage _value)
      (Components|SkinnedMesh|HideBonebyName (Variables|Character|GetMesh) (Utilities|String|StringToName LimbName) "PBO_Term" :!label _label)
      (if (Utilities|Struct|BreakS_LimbData (.Value (Utilities|Map|Find (Variables|LimbData|GetLimbData) LimbName)))
        (Movement|Crawling|StartCrawling)
        (Utilities|Map|Remove (Variables|LimbData|GetLimbData) LimbName))
      (else
        (Utilities|Map|Add _limbhealth LimbName (- _value Damage))))
    (elif (<= _returnvalue_2 0.0)
      (goto _label)
      (else
        (Utilities|Map|Add _limbhealth LimbName _returnvalue_2)))))

(fn StartCrawling
  (bind _capsulecomponent (Variables|Collision|GetCapsuleComponent))
  (Variables|/Script/Engine.CharacterMovementComponent|SetMaxWalkSpeed (Variables|Character|GetCharacterMovement) (Variables|Movement|Crawling|GetDefaultCrawlingSpeed))
  (Components|Capsule|SetCapsuleHalfHeight _capsulecomponent 45.0 true)
  (Transformation|SetRelativeLocation (Variables|Character|GetMesh) "-45.000000, 0,-45.000000" false false)
  (Components|Capsule|SetCapsuleRadius _capsulecomponent 45.0 true)
  (Variables|Movement|Crawling|SetCrawling true))

(fn PlayVoiceSound
  (params (NewSound :type Sound%20Base%20Object%20Reference))
  (bind _voice (Variables|Default|GetVoice))
  (Audio|Components|Audio|SetSound _voice NewSound)
  (Audio|Components|Audio|Play _voice 0.0)
  (Audio|Components|Audio|StopDelayed (Variables|Default|GetVoice_Idle) 0.0)
  (Utilities|Time|SetTimerbyFunctionName self "ResetIdleVoice" 2.0))

(fn ResetIdleVoice
  (Audio|Components|Audio|Play (Variables|Default|GetVoice_Idle) 0.0))

(fn GetPhysicsEffectMaterial
  (return "/Game/Blueprints/Physics/PM_Flesh.PM_Flesh"))

(fn PickUpAmmo
  (params (Type :type E_AmmoType%20Enum :default "NewEnumerator0") (Amount :type Integer))
  (return false))

(fn PickUpHealth
  (params (Health :type Float%20%28single-precision%29))
  (return false))

(fn PickUpHealthItem
  (params (Size :type Integer))
  (return false))

(fn PickUpWeapon
  (params (Weapon :type S%20Weapon%20Structure))
  (return false))