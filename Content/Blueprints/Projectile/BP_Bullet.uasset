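; Bullet projectile that deals point damage to whatever it strikes other than its owner, then destroys itself.
; Blocking hits and collision overlaps are handled separately; overlaps rebuild the hit result at the bullet's location and use the spawn position as damage direction.
; PlayHitEffects asks targets implementing BPI_Interaction for their physics-material effects, then spawns the impact sound and particle system at the bullet.
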(event OnComponentBeginOverlap(CollisionComponent)
  (params (OverlappedComponent :type Primitive%20Component%20Object%20Reference) (OtherActor :type Actor%20Object%20Reference) (OtherComp :type Primitive%20Component%20Object%20Reference) (OtherBodyIndex :type Integer) (bFromSweep :type Boolean) (SweepResult :type Hit%20Result%20Structure%20%28by%20ref%29))
  (bind (_bblockinghit _binitialoverlap _time _distance _location _impactpoint _normal _impactnormal _physmat _hitactor _hitcomponent _hitbonename _hititem _faceindex _tracestart _traceend) (Collision|BreakHitResult SweepResult))
  (bind _returnvalue (Transformation|GetActorLocation))
  (bind _returnvalue_2 (Collision|MakeHitResult _bblockinghit _binitialoverlap _time _distance _returnvalue _returnvalue _normal _impactnormal _physmat _hitactor _hitcomponent _hitbonename _hititem _faceindex _tracestart _traceend))
  (if (!= OtherActor (Components|GetOwner))
    (Utilities|FlowControl|Sequence
      (:then_0
        (Game|Damage|ApplyPointDamage OtherActor (Variables|Default|GetDamage) (Variables|Default|GetStartLocation) _returnvalue_2 0 self "/Game/Blueprints/Projectile/BP_BulletDamage.BP_BulletDamage_C")
        (CallFunction|PlayHitEffects (.ImpactNormal (Collision|BreakHitResult _returnvalue_2)) OtherActor))
      (:then_1
        (Actor|DestroyActor)))))

(event EventBeginPlay
  ;[1 1 1] Begin play
  (Variables|Default|SetStartLocation (Transformation|GetActorLocation)))

(event Collision|EventHit
  (params (MyComp :type Primitive%20Component%20Object%20Reference) (Other :type Actor%20Object%20Reference) (OtherComp :type Primitive%20Component%20Object%20Reference) (bSelfMoved :type Boolean) (HitLocation :type Vector :default "0, 0, 0") (HitNormal :type Vector :default "0, 0, 0") (NormalImpulse :type Vector :default "0, 0, 0") (Hit :type Hit%20Result%20Structure%20%28by%20ref%29))
  (bind _returnvalue (Components|GetOwner))
  ;[1 1 1] Event hit(when bullet hit non-pawn things likes boxes, walls ,etc.)
  (if (!= Other _returnvalue)
    (Utilities|FlowControl|Sequence
      (:then_0
        (bind _returnvalue_2 (Game|Damage|ApplyPointDamage Other (Variables|Default|GetDamage) HitLocation Hit 0 _returnvalue "/Script/Engine.DamageType"))
        (Development|PrintString (Utilities|String|ToString(Float) _returnvalue_2))
        (CallFunction|PlayHitEffects HitLocation Other))
      (:then_1
        (Actor|DestroyActor) ; Then destroy this projectile
      ))))

(fn ConstructionScript)

(fn PlayHitEffects
  (params (InpactNormal :type Vector) (hitActor :type Actor%20Object%20Reference))
  (bind _returnvalue (Transformation|GetActorLocation))
  (if (Utilities|DoesObjectImplementInterface hitActor "/Game/Blueprints/BPI_Interaction.BPI_Interaction_C")
    (bind _mat (Class|BPIInteraction|GetPhysicsEffectMaterial(Message) hitActor))
    (Audio|PlaySoundatLocation (Variables|/Game/Blueprints/Physics/BP_PhysicsMaterial.BP_PhysicsMaterial_C|GetBulletHitEffect _mat) _returnvalue "0, 0, 0" 1.0 1.0 0.0 0 0 0)
    (Niagara|SpawnSystematLocation (Variables|/Game/Blueprints/Physics/BP_PhysicsMaterial.BP_PhysicsMaterial_C|GetHitEffect _mat) _returnvalue (Math|Rotator|FindLookatRotation _returnvalue InpactNormal))))